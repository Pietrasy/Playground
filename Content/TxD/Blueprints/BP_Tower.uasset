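; BP_Tower is a turret that targets BP_Enemy actors entering its Range-sized sphere and fires at them.
; Overlap begin and end toggle Tick, which yaws the cannon toward the target and starts firing through a DoOnce.
; StartFire draws randomly from a projectile pool spawned at BeginPlay, teleporting and shooting projectiles, and sets a looping FireDelay timer.
; Damage comes from a line trace to the target's location, sent as a HitEnemy message.
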(event OnComponentBeginOverlap(RangeSphere)
  (params (OverlappedComponent :type Primitive%20Component%20Object%20Reference) (OtherActor :type Actor%20Object%20Reference) (OtherComp :type Primitive%20Component%20Object%20Reference) (OtherBodyIndex :type Integer) (bFromSweep :type Boolean) (SweepResult :type Hit%20Result%20Structure%20%28by%20ref%29))
  (bind _asbp_enemy (Utilities|Casting|CastToBP_Enemy OtherActor))
  (Variables|Default|SetTarget _asbp_enemy)
  (Actor|Tick|SetActorTickEnabled true))

(event OnComponentEndOverlap(RangeSphere)
  (params (OverlappedComponent :type Primitive%20Component%20Object%20Reference) (OtherActor :type Actor%20Object%20Reference) (OtherComp :type Primitive%20Component%20Object%20Reference) (OtherBodyIndex :type Integer))
  (bind _asbp_enemy (Utilities|Casting|CastToBP_Enemy OtherActor))
  (Variables|Default|SetTarget _asbp_enemy)
  (Actor|Tick|SetActorTickEnabled false))

(event Custom|StartFire
  (bind _projectiles (Variables|Default|GetProjectiles))
  (bind _outitem (Utilities|Array|Random _projectiles))
  (Variables|Default|SetStorageTransform (Transformation|GetWorldTransform (Variables|Default|GetProjectileStorage)))
  (Transformation|SetActorLocation _outitem (Transformation|GetWorldLocation (Variables|Default|GetFireSpot)) false true)
  (Default|Shoot _outitem)
  (bind _outhit (Collision|LineTraceByChannel (Transformation|GetWorldLocation (Variables|Default|GetFireSpot)) (Variables|Default|GetTargetLocation) "TraceTypeQuery1" false 0 "ForDuration"))
  (Class|BPIEnemy|HitEnemy(Message) (.hitactor _outhit) (Variables|Default|GetDamage))
  (Utilities|Time|SetTimerbyEvent (EventDispatchers|CreateEvent :!event Custom|StartFire) (Variables|Default|GetFireDelay) true)
  (Development|PrintString "Spawn"))

(event EventTick
  (params (DeltaSeconds :type Float%20%28single-precision%29))
  (Variables|Default|SetTargetLocation (Transformation|GetActorLocation (Variables|Default|GetTarget)))
  (Variables|Default|SetRotatorToTarget (Math|Rotator|MakeRotfromX (- (Variables|Default|GetTargetLocation) (Transformation|GetWorldLocation (Variables|Default|GetCannon)))))
  (Transformation|SetRelativeRotation (Variables|Default|GetCannon) (Class|KismetMathLibrary|RInterptoConstant (Variables|/Script/Engine.SceneComponent|GetRelativeRotation (Variables|Default|GetCannon)) (Math|Rotator|MakeRotator 0.0 0.0 (.Yaw (Math|Rotator|BreakRotator (Variables|Default|GetRotatorToTarget)))) DeltaSeconds 1e+03) false false)
  (Utilities|FlowControl|DoOnce false
    (:Completed
      (CallFunction|StartFire))))

(event EventBeginPlay
  (Variables|Default|SetStorageTransform (Transformation|GetWorldTransform (Variables|Default|GetProjectileStorage)))
  (for _index (range 0 (- (Variables|Default|GetNumberProjectilesToSpawnAtPool) 1))
    (CallFunction|SpawnProjectile)))

(fn ConstructionScript
  (Components|Sphere|SetSphereRadius (Variables|Default|GetRangeSphere) (Variables|Default|GetRange) true))

(fn SpawnProjectile
  (bind _returnvalue (Game|SpawnActorfromClass (Variables|Default|GetProjectileType) (Variables|Default|GetStorageTransform) "Undefined" "MultiplyWithRoot" 0 0))
  (Utilities|Array|AddUnique (Variables|Default|GetProjectiles) _returnvalue)
  (return))