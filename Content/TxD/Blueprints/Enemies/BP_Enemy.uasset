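; Enemy actor that travels along a Route spline and reports back to its Spawner.
; MoveEnemy scales a timeline's play rate by Speed, then maps its interpolation to spline distance to update world location.
; Reaching the end or the destroy event notifies the Spawner through UptadeEnemy.
; HitEnemy only prints the damage, and construction applies the Color material to the Body.
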(event Custom|OnDestroyEnemy
  ;[0.2 0.75 0.2] On destroy enemy
  (CallFunction|UptadeEnemy))

(event Custom|MoveEnemy
  ;[0.2 0.75 0.2] Move enemy
  (CallFunction|SetSpeedEnemyMovement (Variables|Default|GetSpeed))
  (bind _interpolation (Timeline|MoveAlongSpline PlayFromStart)
    (:Update
      (bind _output_get (Variables|Default|SetVelocityTemp (Spline|GetLocationatDistanceAlongSpline (Variables|/Game/TxD/Blueprints/BP_Route.BP_Route_C|GetRoute (Variables|Default|GetRoute)) (Math|Float|Lerp 0.0 (Spline|GetSplineLength (Variables|/Game/TxD/Blueprints/BP_Route.BP_Route_C|GetRoute (Variables|Default|GetRoute))) _interpolation) "World")))
      (Transformation|SetActorTransform (Math|Transform|MakeTransform _output_get "0, 0, 0" "1.000000,1.000000,1.000000")))
    (:Finished
      (CallFunction|UptadeEnemy))))

(event EventHitEnemy
  (params (Damage :type Integer))
  (Development|PrintString (Utilities|String|Append "Hit damage: " (Utilities|String|ToString(Integer) Damage))))

(fn ConstructionScript
  (Rendering|Material|SetMaterial (Variables|Default|GetBody) 0 (Variables|Default|GetColor)))

(fn SetSpeedEnemyMovement
  (params (Speed :type Float%20%28double-precision%29))
  (Components|Timeline|SetPlayRate (Variables|Default|GetMoveAlongSpline) (* Speed 0.1)))

(fn UptadeEnemy
  (Default|UptadeEnemy (Variables|Default|GetSpawner))
  (return))