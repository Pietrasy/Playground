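; BP_Enemy is an enemy actor that travels from start to end along the spline of its assigned Route.
; MoveEnemy scales Speed into the play rate of a timeline, whose interpolation value sets the actor's world location by distance along the spline.
; Reaching the end or the OnDestroyEnemy event makes the Spawner count enemies.
; The construction script applies the Color material to the Body.
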(event Custom|OnDestroyEnemy
  ;[0.2 0.75 0.2] On destroy enemy
  (Default|CountEnemies (Variables|Default|GetSpawner)))

(event Custom|MoveEnemy
  ;[0.2 0.75 0.2] Move enemy
  (CallFunction|SetSpeedEnemyMovement (Variables|Default|GetSpeed))
  (bind _interpolation (Timeline|MoveAlongSpline PlayFromStart)
    (:Update
      (Transformation|SetActorTransform (Math|Transform|MakeTransform (Spline|GetLocationatDistanceAlongSpline (Variables|/Game/TxD/Blueprints/BP_Route.BP_Route_C|GetRoute (Variables|Default|GetRoute)) (Math|Float|Lerp 0.0 (Spline|GetSplineLength (Variables|/Game/TxD/Blueprints/BP_Route.BP_Route_C|GetRoute (Variables|Default|GetRoute))) _interpolation) "World") "0, 0, 0" "1.000000,1.000000,1.000000")))
    (:Finished
      (Default|CountEnemies (Variables|Default|GetSpawner)))))

(fn ConstructionScript
  (Rendering|Material|SetMaterial (Variables|Default|GetBody) 0 (Variables|Default|GetColor)))

(fn SetSpeedEnemyMovement
  (params (Speed :type Float%20%28double-precision%29))
  (Components|Timeline|SetPlayRate (Variables|Default|GetMoveAlongSpline) (* Speed 0.1)))