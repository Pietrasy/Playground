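; Projectile actor for a tower defense game, with a configurable static mesh applied on BeginPlay.
; Shoot sets the projectile movement velocity from a scaled direction, activates the movement component, then calls StopTime on the tower defense player controller.
; Overlap with an enemy only prints a debug string, with no damage or destruction logic.
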(event OnComponentBeginOverlap(Projectile)
  (params (OverlappedComponent :type Primitive%20Component%20Object%20Reference) (OtherActor :type Actor%20Object%20Reference) (OtherComp :type Primitive%20Component%20Object%20Reference) (OtherBodyIndex :type Integer) (bFromSweep :type Boolean) (SweepResult :type Hit%20Result%20Structure%20%28by%20ref%29))
  (Utilities|Casting|CastToBP_Enemy OtherActor)
  (Development|PrintString "Hello"))

(event Custom|Shoot
  (params (Direction :type Vector))
  (Variables|/Script/Engine.MovementComponent|SetVelocity (Variables|Default|GetProjectileMovement) (* Direction 1e+01))
  (Components|Activation|Activate (Variables|Default|GetProjectileMovement) false)
  (bind _aspc_tower_defense (Utilities|Casting|CastToPC_TowerDefense (Game|GetPlayerController 0)))
  (Default|StopTime _aspc_tower_defense))

(event EventBeginPlay
  (Components|StaticMesh|SetStaticMesh (Variables|Default|GetProjectile) (Variables|Default|GetProjectileStaticMesh)))

(fn ConstructionScript)