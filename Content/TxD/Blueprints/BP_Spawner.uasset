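; Tower defense spawner that pre-spawns the current wave's enemies into a pool and releases them onto a route.
; On BeginPlay it reads the wave's enemy classes from GM_TowerDefense, spawns them at the Pool transform with Spawner and Route references, and starts a looping timer.
; PutEnemyAtSpline moves the first pooled enemy to the spawn point, starts its movement and removes it from the pool.
; AddEnemyToArray returns an enemy to the pool, then immediately calls PutEnemyAtSpline.
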(event Custom|PutEnemyAtSpline
  ;[0.2 0.75 0.2] Put enemy at spline
  (|CheckIfArrayIsEmpty)
  (bind _enemy (CallFunction|GetEnemyfromArray))
  (Transformation|SetActorLocation _enemy (Variables|Default|GetSpawnPointLocation) false false)
  (Default|MoveObject (Variables|Default|GetEnemy))
  (Utilities|Array|RemoveItem (Variables|Default|GetEnemiesInPool) (Variables|Default|GetEnemy)))

(event Custom|SpawnEnemiesInPool
  ;[0.2 0.75 0.2] Spawn enemies in pool
  (CallFunction|SpawnEnemyinPool))

(event Custom|AddEnemyToArray
  (params (Enemy :type BP%20Enemy%20Object%20Reference))
  ;[0.2 0.75 0.2] Add enemy to array
  (Utilities|Array|AddUnique (Variables|Default|GetEnemiesInPool) Enemy)
  (CallFunction|PutEnemyatSpline))

(event EventBeginPlay
  ;[0.2 0.75 0.2] Begin play
  (bind _asgm_tower_defense (Utilities|Casting|CastToGM_TowerDefense (Game|GetGameMode)))
  (Variables|Default|SetGameMode _asgm_tower_defense)
  (Variables|Default|SetEnemiesToSpawn (.enemies (.Value (Utilities|Map|Find (.wave (Variables|/Game/TxD/Blueprints/Core/GM_TowerDefense.GM_TowerDefense_C|GetWaves (Variables|Default|GetGameMode))) (Variables|/Game/TxD/Blueprints/Core/GM_TowerDefense.GM_TowerDefense_C|GetCurrentWave (Variables|Default|GetGameMode))))))
  (CallFunction|SetPoolTransform)
  (CallFunction|SpawnEnemiesinPool)
  (CallFunction|SetPointLocation)
  (bind _returnvalue (Utilities|Time|SetTimerbyEvent (EventDispatchers|CreateEvent :!event Custom|PutEnemyAtSpline) (Variables|Default|GetTimeToSpawn) true))
  (Variables|Default|SetPutEnemyAtSpline_TimerHandle _returnvalue))

(fn ConstructionScript)

(fn SetPoolTransform
  (bind _output_get (Variables|Default|SetPoolTransform (Transformation|GetWorldTransform (Variables|Default|GetPool))))
  (return _output_get))

(fn SetPointLocation
  (bind _output_get (Variables|Default|SetSpawnPointLocation (Transformation|GetWorldLocation (Variables|Default|GetSpawnPoint))))
  (return _output_get))

(fn SpawnEnemyinPool
  (for _array_element (Variables|Default|GetEnemiesToSpawn)
    (bind _returnvalue (Game|SpawnActorfromClass _array_element (Variables|Default|GetPoolTransform) "Undefined" "MultiplyWithRoot" 0 0))
    (bind _output_get (LocalVariables|SetSpawnedEnemy _returnvalue))
    (Variables|/Game/TxD/Blueprints/BP_Enemy.BP_Enemy_C|SetSpawner _output_get self)
    (Variables|/Game/TxD/Blueprints/BP_Enemy.BP_Enemy_C|SetRoute (LocalVariables|GetSpawnedEnemy) (Variables|Default|GetRoute))
    (Utilities|Array|AddUnique (Variables|Default|GetEnemiesInPool) (LocalVariables|GetSpawnedEnemy)))
  (return))

(fn GetEnemyfromArray
  (for _array_element (Variables|Default|GetEnemiesInPool)
    (bind _output_get (Variables|Default|SetEnemy _array_element))
    (return _output_get)))