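; Tower defense game mode that tracks wave progression and end of game.
; On BeginPlay it caches the player controller, HUD and the level's wave manager actor, then shows the mouse cursor.
; EndWave shows the HUD button while waves remain, otherwise flags and prints game over.
; NextWave advances the wave count, updates the HUD counter and tells the wave manager to select the next wave.
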(event EventBeginPlay
  (CallFunction|SetPlayerController)
  (CallFunction|SetHUD)
  (CallFunction|SetWaveManager)
  (Variables|/Script/Engine.PlayerController|SetbShowMouseCursor (Variables|Default|GetPlayerController) true))

(fn ConstructionScript)

(fn EndWave
  (if (> (Utilities|Map|Length (.wave (Variables|Default|GetWaves))) (Variables|Default|GetCurrentWave))
    (Default|ShowButton (Variables|/Game/TxD/Blueprints/Core/HUD_TowerDefense.HUD_TowerDefense_C|GetWidgetUI (Variables|Default|GetHUD)))
    (else
      (Variables|Default|SetIsEndGame true)
      (Development|PrintString "End Game!"))))

(fn NextWave
  (Math|Integer|IncrementInt (Variables|Default|GetCurrentWave)
    (:%20%20
      (Default|UptadeCounter (Variables|Default|GetHUD))
      (Default|SelectNextWave (Variables|Default|GetWaveMenager)))))

(fn SetPlayerController
  (bind _aspc_tower_defense (Utilities|Casting|CastToPC_TowerDefense (Game|GetPlayerController 0)))
  (Variables|Default|SetPlayerController _aspc_tower_defense)
  (return))

(fn SetHUD
  (bind _ashud_tower_defense (Utilities|Casting|CastToHUD_TowerDefense (HUD|GetHUD (Game|GetPlayerController 0))))
  (Variables|Default|SetHUD _ashud_tower_defense)
  (return))

(fn SetWaveManager
  (bind _returnvalue (Actor|GetActorOfClass "/Game/TxD/Blueprints/BP_WaveMenager.BP_WaveMenager_C"))
  (Variables|Default|SetWaveMenager _returnvalue))