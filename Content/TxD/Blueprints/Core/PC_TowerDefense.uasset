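; Player controller for the tower defense game that controls game speed through global time dilation.
; BeginPlay starts the game at half speed, and keyboard keys step the speed up or down, reset it to normal, or set it to zero.
; A StopTime function slows time to a near halt.
; Every change writes the Speed variable and applies it immediately, with no clamping on the increments.
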(event EventBeginPlay
  (bind _output_get (Variables|Default|SetSpeed 0.5))
  (Utilities|Time|SetGlobalTimeDilation _output_get))

(event Input|KeyboardEvents|Add
  (params (Key :type Key%20Structure :default "None"))
  (:Pressed
    (bind _output_get (Variables|Default|SetSpeed (+ (Variables|Default|GetSpeed) 0.1)))
    (Utilities|Time|SetGlobalTimeDilation _output_get)))

(event Input|KeyboardEvents|Subtract
  (params (Key :type Key%20Structure :default "None"))
  (:Pressed
    (bind _output_get (Variables|Default|SetSpeed (- (Variables|Default|GetSpeed) 0.1)))
    (Utilities|Time|SetGlobalTimeDilation _output_get)))

(event Input|KeyboardEvents|NumPadZero
  (params (Key :type Key%20Structure :default "None"))
  (:Pressed
    (bind _output_get (Variables|Default|SetSpeed 1.0))
    (Utilities|Time|SetGlobalTimeDilation _output_get)))

(event Input|KeyboardEvents|SpaceBar
  (params (Key :type Key%20Structure :default "None"))
  (:Pressed
    (bind _output_get (Variables|Default|SetSpeed 0.0))
    (Utilities|Time|SetGlobalTimeDilation _output_get)))

(fn ConstructionScript)

(fn StopTime
  (bind _output_get (Variables|Default|SetSpeed 0.005))
  (Utilities|Time|SetGlobalTimeDilation _output_get))