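; Tower actor that fires pooled projectiles at BP_Enemy actors entering its range sphere, which is sized from Range.
; BeginPlay pre-spawns projectiles at a storage point; each shot moves a random one to the fire spot.
; StartFire aims the cannon using distance-scaled velocity lead, but shoots along the flattened direction to the target's current position.
; It also draws a debug trace and sets a looping FireDelay timer, which range exit never clears.
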(event OnComponentBeginOverlap(RangeSphere)
  (params (OverlappedComponent :type Primitive%20Component%20Object%20Reference) (OtherActor :type Actor%20Object%20Reference) (OtherComp :type Primitive%20Component%20Object%20Reference) (OtherBodyIndex :type Integer) (bFromSweep :type Boolean) (SweepResult :type Hit%20Result%20Structure%20%28by%20ref%29))
  (bind _asbp_enemy (Utilities|Casting|CastToBP_Enemy OtherActor))
  (Variables|Default|SetTarget _asbp_enemy)
  (Variables|Default|SetTargetLocation (Transformation|GetActorLocation (Variables|Default|GetTarget)))
  (bind _output_get (Variables|Default|SetRotatorToTarget (Math|Rotator|MakeRotfromX (- (Variables|Default|GetTargetLocation) (Transformation|GetWorldLocation (Variables|Default|GetCannon))))))
  (Transformation|SetRelativeRotation (Variables|Default|GetCannon) _output_get false false)
  (Actor|Tick|SetActorTickEnabled true)
  (CallFunction|StartFire))

(event OnComponentEndOverlap(RangeSphere)
  (params (OverlappedComponent :type Primitive%20Component%20Object%20Reference) (OtherActor :type Actor%20Object%20Reference) (OtherComp :type Primitive%20Component%20Object%20Reference) (OtherBodyIndex :type Integer))
  (bind _asbp_enemy (Utilities|Casting|CastToBP_Enemy OtherActor))
  (Variables|Default|SetTarget _asbp_enemy)
  (Actor|Tick|SetActorTickEnabled false))

(event Custom|StartFire
  (bind _cannon (Variables|Default|GetCannon))
  (bind _returnvalue (Transformation|GetWorldLocation _cannon))
  (Utilities|FlowControl|Sequence
    (:then_0
      (Variables|Default|SetTargetLocation (Transformation|GetActorLocation (Variables|Default|GetTarget)))
      (Variables|Default|SetRotatorToTarget (Math|Rotator|MakeRotfromX (- (Math|Vector|MakeVector (.x (Variables|Default|GetTargetLocation)) (.y (Variables|Default|GetTargetLocation)) (.z _returnvalue)) (Math|Vector|MakeVector (.x _returnvalue) (.y _returnvalue) (.z _returnvalue)))))
      (Transformation|SetRelativeRotation (Variables|Default|GetCannon) (Math|Rotator|FindLookatRotation (Transformation|GetWorldLocation (Variables|Default|GetBase)) (+ (Variables|Default|GetTargetLocation) (* (/ (Transformation|GetDistanceTo (Variables|Default|GetTarget)) 1.0) (Variables|/Game/TxD/Blueprints/Enemies/BP_Enemy.BP_Enemy_C|GetVelocityTemp (Variables|Default|GetTarget))))) false false))
    (:then_1
      (Variables|Default|SetProjectileFromClip (.OutItem (Utilities|Array|Random (Variables|Default|GetProjectiles))))
      (Transformation|SetActorLocation (Variables|Default|GetProjectileFromClip) (Transformation|GetWorldLocation (Variables|Default|GetFireSpot)) false false)
      (Default|Shoot (Variables|Default|GetProjectileFromClip) (- (Math|Vector|MakeVector (.x (Variables|Default|GetTargetLocation)) (.y (Variables|Default|GetTargetLocation)) (.z _returnvalue)) (Math|Vector|MakeVector (.x _returnvalue) (.y _returnvalue) (.z _returnvalue))))
      (|CastTrace)
      (Utilities|Time|SetTimerbyEvent (EventDispatchers|CreateEvent :!event Custom|StartFire) (Variables|Default|GetFireDelay) true))))

(event EventTick
  (params (DeltaSeconds :type Float%20%28single-precision%29)))

(event EventBeginPlay
  (Variables|Default|SetStorageTransform (Transformation|GetWorldTransform (Variables|Default|GetProjectileStorage)))
  (for _index (range 0 (- (Variables|Default|GetNumberProjectilesToSpawnAtPool) 1))
    (CallFunction|SpawnProjectile)))

(fn ConstructionScript
  (Components|Sphere|SetSphereRadius (Variables|Default|GetRangeSphere) (Variables|Default|GetRange) true))

(fn SpawnProjectile
  (bind _returnvalue (Game|SpawnActorfromClass (Variables|Default|GetProjectileType) (Variables|Default|GetStorageTransform) "Undefined" "MultiplyWithRoot" 0 0))
  (Utilities|Array|AddUnique (Variables|Default|GetProjectiles) _returnvalue)
  (return))