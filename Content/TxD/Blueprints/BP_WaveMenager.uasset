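; Wave manager for a tower defense game that loads the current wave's enemy list and detects when the wave is over.
; On BeginPlay it caches GM_TowerDefense and the level's BP_Spawner, then looks up the wave's enemies in the game mode's wave map by CurrentWave.
; UptadeWaveState counts passed enemies; once the count reaches the wave size, it has the spawner clean up and the game mode end the wave.
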(event Custom|UptadeWaveState
  (bind _result (Math|Integer|IncrementInt (Variables|Default|GetPassedEnemies))
    (:%20%20
      (if (>= _result (Variables|Default|GetNumberEnemiesInCurrentWave))
        (Default|CleanBeforeNextWave (Variables|Default|GetSpawner))
        (Default|EndWave (Variables|Default|GetGameMode))))))

(event EventBeginPlay
  (CallFunction|SetGameMode)
  (CallFunction|SetSpawner)
  (CallFunction|SelectNextWave))

(fn ConstructionScript)

(fn SetGameMode
  (bind _asgm_tower_defense (Utilities|Casting|CastToGM_TowerDefense (Game|GetGameMode)))
  (Variables|Default|SetGameMode _asgm_tower_defense)
  (return))

(fn SelectNextWave
  (bind _output_get (Variables|Default|SetEnemiesToSpawn (.enemies (.Value (Utilities|Map|Find (.wave (Variables|/Game/TxD/Blueprints/Core/GM_TowerDefense.GM_TowerDefense_C|GetWaves (Variables|Default|GetGameMode))) (Variables|/Game/TxD/Blueprints/Core/GM_TowerDefense.GM_TowerDefense_C|GetCurrentWave (Variables|Default|GetGameMode)))))))
  (Variables|Default|SetNumberEnemiesInCurrentWave (Utilities|Array|Length _output_get))
  (return))

(fn SetSpawner
  (bind _returnvalue (Actor|GetActorOfClass "/Game/TxD/Blueprints/BP_Spawner.BP_Spawner_C"))
  (Variables|Default|SetSpawner _returnvalue)
  (return))