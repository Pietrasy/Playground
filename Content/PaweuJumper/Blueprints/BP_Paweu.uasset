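; BP_Paweu is an actor that moves itself along its forward vector while aiming an arrow component at the hook.
; On BeginPlay it starts the Movement timeline, whose updates offset the location by Speed scaled by the interpolation track, without sweep.
; Each update first calls FaceArrowToHook, which looks up BP_Hook by class and applies the world-space look-at rotation as the Arrow's relative rotation.
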(event EventBeginPlay
  (bind _returnvalue (Transformation|GetActorLocation))
  (bind _inerpolation (Timeline|Movement PlayFromStart)
    (:Update
      (CallFunction|FaceArrowtoHook)
      (Transformation|SetActorLocation (Math|Vector|Lerp(Vector) _returnvalue (+ _returnvalue (* (Transformation|GetActorForwardVector) (Variables|Default|GetSpeed))) _inerpolation) false false))))

(fn ConstructionScript)

(fn FaceArrowtoHook
  (bind _returnvalue (Actor|GetActorOfClass "/Game/PaweuJumper/Blueprints/BP_Hook.BP_Hook_C"))
  (Transformation|SetRelativeRotation (Variables|Default|GetArrow) (Math|Rotator|FindLookatRotation (Transformation|GetWorldLocation (Variables|Default|GetArrow)) (Transformation|GetActorLocation _returnvalue)) false false))